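; BP_TunnelSpawner builds a chain of BP_Tunnel segments, each populated with an enemy or health pack.
; On BeginPlay it clears existing tunnels, enemies and health packs, then spawns a few segments starting at the player pawn.
; Each following segment attaches at the newest tunnel's SpawnPoint.
; Every tunnel receives a spawner reference and randomized wall, plus a coin-flip enemy or health pack offset along X.
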(event `self.ReceiveBeginPlay`
  (`self.Spawn Initial Tunnels`))

(event `self.ReceiveActorBeginOverlap`
  (params (OtherActor :type "Actor Object Reference")))

(event `self.ReceiveTick`
  (params (DeltaSeconds :type "Float (single-precision)")))

(fn `Spawn Initial Tunnels`
  (`|ExecutionSequence`
    (:`then_0`
      (bind _outactors (`GameplayStatics.GetAllActorsOfClass` "/Game/InfiniteMatrix/Blueprints/BP_Tunnel.BP_Tunnel_C"))
      (for _array_element _outactors
        (`self.K2_DestroyActor` _array_element)))
    (:`then_1`
      (bind _outactors_2 (`GameplayStatics.GetAllActorsOfClass` "/Game/InfiniteMatrix/Blueprints/BP_HealthPack.BP_HealthPack_C"))
      (for _array_element_2 _outactors_2
        (`self.K2_DestroyActor` _array_element_2)))
    (:`then_2`
      (bind _outactors_3 (`GameplayStatics.GetAllActorsOfClass` "/Game/InfiniteMatrix/Blueprints/BP_Enemy.BP_Enemy_C"))
      (for _array_element_3 _outactors_3
        (`self.K2_DestroyActor` _array_element_3)))
    (:`then_3`
      (for _ (range 3)
        (`/Engine/EditorBlueprintResources/StandardMacros.IsValid` (`self.Newest Tunnel`)
          (:`Is Valid`
            (`self.Spawn Tunnel at Spawn Point`))
          (:`Is Not Valid`
            (`self.Spawn Tunnel` (`self.K2_GetActorLocation` (`GameplayStatics.GetPlayerPawn` 0)))))))))

(fn `Spawn Tunnel`
  (params (`Spawn Location` :type "Vector Structure"))
  (bind _returnvalue (`KismetMathLibrary.MakeVector` (+ (.x `Spawn Location`) 1000.0) (.y `Spawn Location`) (.z `Spawn Location`)))
  (`|ExecutionSequence`
    (:`then_0`
      (bind _returnvalue_2 (`|SpawnActorFromClass` "/Game/InfiniteMatrix/Blueprints/BP_Tunnel.BP_Tunnel_C" (`KismetMathLibrary.MakeTransform` `Spawn Location`) "Undefined" "OverrideRootScale" null null))
      (bind _output_get (set `self.Newest Tunnel` _returnvalue_2))
      (set `/Game/InfiniteMatrix/Blueprints/BP_Tunnel.Tunnel Spawner` self _output_get)
      (`/Game/InfiniteMatrix/Blueprints/BP_Tunnel.Randomize Wall` _output_get))
    (:`then_1`
      (if (`KismetMathLibrary.RandomBool`)
        (`|SpawnActorFromClass` "/Game/InfiniteMatrix/Blueprints/BP_Enemy.BP_Enemy_C" (`KismetMathLibrary.MakeTransform` _returnvalue) "Undefined" "OverrideRootScale" null null)
        (else
          (`|SpawnActorFromClass` "/Game/InfiniteMatrix/Blueprints/BP_HealthPack.BP_HealthPack_C" (`KismetMathLibrary.MakeTransform` _returnvalue) "Undefined" "OverrideRootScale" null null))))))

(fn `Spawn Tunnel at Spawn Point`
  (`self.Spawn Tunnel` (`SceneComponent.K2_GetComponentLocation` (`/Game/InfiniteMatrix/Blueprints/BP_Tunnel.SpawnPoint` (`self.Newest Tunnel`)))))

(fn `UserConstructionScript`)