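; BP_Projectile is the player-relative projectile in Infinite Matrix that destroys enemies for score.
; Each Tick it sweeps along world X by the player's CurrentSpeed plus a fixed offset, without delta-time scaling, so it outpaces the player.
; When its Sphere hits anything it destroys itself, and if the other actor is exactly BP_Enemy it destroys that too and adds points through the player's ScoreWidget.
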(event `self.ReceiveTick`
  (params (DeltaSeconds :type "Float (single-precision)"))
  (bind _asbp_player (cast `/Game/InfiniteMatrix/Blueprints/BP_Player` (`GameplayStatics.GetPlayerPawn` 0)))
  (`self.K2_AddActorWorldOffset` (`KismetMathLibrary.MakeVector` (+ (`/Game/InfiniteMatrix/Blueprints/BP_Player.Current Speed` _asbp_player) 50.0)) true))

(event `self.Sphere.OnComponentHit`
  (params (HitComponent :type "PrimitiveComponent Object Reference") (OtherActor :type "Actor Object Reference") (OtherComp :type "PrimitiveComponent Object Reference") (NormalImpulse :type "Vector Structure") (Hit :type "HitResult Structure (by ref)"))
  (`self.K2_DestroyActor`)
  (if (== (`GameplayStatics.GetObjectClass` OtherActor) "/Game/InfiniteMatrix/Blueprints/BP_Enemy.BP_Enemy_C")
    (`self.K2_DestroyActor` OtherActor)
    (bind _asbp_player (cast `/Game/InfiniteMatrix/Blueprints/BP_Player` (`GameplayStatics.GetPlayerPawn` 0)))
    (`/Game/InfiniteMatrix/UI/WBP_Score.Update Score` (`/Game/InfiniteMatrix/Blueprints/BP_Player.Score Widget` _asbp_player) 250)))

(fn `UserConstructionScript`)