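; BP_HealthPack is a spinning pickup that heals the player on contact.
; It starts at a random rotation, then turns on all three axes each Tick at RotateSpeed.
; A Hitbox overlap with BP_Player calls Heal directly on the player's HealthWidget and destroys the pack.
; Tick also destroys the pack once its world X falls below the player pawn's, cleaning up missed pickups.
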(event `self.ReceiveBeginPlay`
  (bind _returnvalue (`KismetMathLibrary.RandomFloatInRange` 0.0 360.0))
  (`self.K2_AddActorWorldRotation` (`KismetMathLibrary.MakeRotator` _returnvalue _returnvalue _returnvalue)))

(event `self.ReceiveTick`
  (params (DeltaSeconds :type "Float (single-precision)"))
  (bind _returnvalue_x (`KismetMathLibrary.BreakVector` (`self.K2_GetActorLocation`)))
  (bind _returnvalue_x_2 (`KismetMathLibrary.BreakVector` (`self.K2_GetActorLocation` (`GameplayStatics.GetPlayerPawn` 0))))
  (bind _returnvalue (* DeltaSeconds (`self.Rotate Speed`)))
  (`self.K2_AddActorWorldRotation` (`KismetMathLibrary.MakeRotator` _returnvalue _returnvalue _returnvalue))
  (if (< _returnvalue_x _returnvalue_x_2)
    (`self.K2_DestroyActor`)))

(event `self.Hitbox.OnComponentBeginOverlap`
  (params (OverlappedComponent :type "PrimitiveComponent Object Reference") (OtherActor :type "Actor Object Reference") (OtherComp :type "PrimitiveComponent Object Reference") (OtherBodyIndex :type Integer) (bFromSweep :type Boolean) (SweepResult :type "HitResult Structure (by ref)"))
  (bind _asbp_player (cast `/Game/InfiniteMatrix/Blueprints/BP_Player` OtherActor))
  (`/Game/InfiniteMatrix/UI/WBP_Health.Heal` (`/Game/InfiniteMatrix/Blueprints/BP_Player.Health Widget` _asbp_player))
  (`self.K2_DestroyActor`))

(fn `UserConstructionScript`)